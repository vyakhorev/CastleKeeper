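; CloseEnough is a Behavior Tree decorator for enemy mobs that gates a branch on distance to the followed target.
; It casts its owner to MobAIController_BP and measures from the controlled pawn to the TragetToFollow blackboard actor.
; Despite the name, the condition passes when that distance is at least AcceptableDistance, meaning the mob is not yet close.
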(fn `PerformConditionCheck`
  (params (OwnerActor :type "Actor Object Reference"))
  (returns (ReturnValue :type Boolean))
  (bind _asmob_aicontroller_bp (cast `/Game/CastleKeeperLogic/Blueprints/Enemy/MobAIController_BP` OwnerActor))
  (set `self.AI_CON_Ref` _asmob_aicontroller_bp)
  (return (>= (`KismetMathLibrary.VSize` (- (`Actor.K2_GetActorLocation` (`BTFunctionLibrary.GetBlackboardValueAsActor` (`self.TragetToFollow`))) (`Actor.K2_GetActorLocation` (`Controller.K2_GetPawn` (`self.AI_CON_Ref`))))) (`self.AcceptableDistance`))))
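; Enemy AI aggro check that points the blackboard target at Crystall actors.
; Each tick it loops over all Crystall actors and writes each to TargetToFollow and its position to TargetLocation, so the last one wins.
; An older sphere-trace and line-of-sight detection path that ignores AngryTrolls is left disconnected and never runs, despite the graph comment describing it.
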(event `self.ReceiveTick`
  (params (OwnerActor :type "Actor Object Reference") (DeltaSeconds :type "Float (single-precision)"))
  ;[1 1 1] Cast spheres, checks line of sight, sets values to blackboard
  (bind _outactors (`GameplayStatics.GetAllActorsOfClass` "/Game/CastleKeeperLogic/Blueprints/Castle/Crystall.Crystall_C"))
  (for _array_element _outactors
    (`BTFunctionLibrary.SetBlackboardValueAsObject` (`self.TargetToFollow`) _array_element)
    (`BTFunctionLibrary.SetBlackboardValueAsVector` (`self.TargetLocation`) (`Actor.K2_GetActorLocation` _array_element))))
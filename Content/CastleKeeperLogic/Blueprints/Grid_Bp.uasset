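; Grid actor that shows a Rand_Sprite_BP on the 100-unit grid position under the player's mouse cursor.
; Tick accumulates time and, about every 0.05 seconds, traces under the cursor on Visibility, offsetting and truncating X and Y to the grid with Z flattened to zero.
; It spawns a fresh sprite there and destroys the previous one rather than moving it, printing debug strings along the way.
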(event `self.ReceiveTick`
  (params (DeltaSeconds :type "Float (single-precision)"))
  (bind _current_sprite (`self.current_sprite`))
  (bind _returnvalue (`KismetMathLibrary.MakeVector` (* (`KismetMathLibrary.FTrunc` (/ (- (.x (`.Location` (`GameplayStatics.BreakHitResult` (`PlayerController.GetHitResultUnderCursorByChannel` (`GameplayStatics.GetPlayerController` 0) "TraceTypeQuery1" true)))) 50.0) 100.0)) 100.0) (* (`KismetMathLibrary.FTrunc` (/ (- (.y (`.Location` (`GameplayStatics.BreakHitResult` (`PlayerController.GetHitResultUnderCursorByChannel` (`GameplayStatics.GetPlayerController` 0) "TraceTypeQuery1" true)))) 50.0) 100.0)) 100.0) (* (.z (`.Location` (`GameplayStatics.BreakHitResult` (`PlayerController.GetHitResultUnderCursorByChannel` (`GameplayStatics.GetPlayerController` 0) "TraceTypeQuery1" true)))) 0.0)))
  (bind _output_get (set `self.Counter` (+ DeltaSeconds (`self.Counter`))))
  (`/Engine/EditorBlueprintResources/StandardMacros.CompareFloat` _output_get 0.05
    (:`>`
      (`KismetSystemLibrary.PrintString` (`KismetStringLibrary.Conv_VectorToString` _returnvalue))
      (bind _returnvalue_2 (`|SpawnActorFromClass` "/Game/CastleKeeperLogic/Blueprints/Rand_Sprite_BP.Rand_Sprite_BP_C" (`KismetMathLibrary.Conv_VectorToTransform` _returnvalue) "Undefined" "OverrideRootScale" null null))
      (set `self.Counter` 0.0)
      (`/Engine/EditorBlueprintResources/StandardMacros.IsValid` (`self.current_sprite`)
        (:`Is Valid`
          (`self.K2_DestroyActor` _current_sprite)
          (`KismetSystemLibrary.PrintString` (`KismetStringLibrary.Concat_StrStr` "Deleting" (`KismetStringLibrary.Conv_ObjectToString` (`Actor.RootComponent` _current_sprite)))))
        (:`Is Not Valid`
          (`KismetSystemLibrary.PrintString` "notValid")))
      (bind _output_get_2 (set `self.current_sprite` _returnvalue_2))
      (`KismetSystemLibrary.PrintString` (`KismetSystemLibrary.GetDisplayName` _output_get_2)))))

(fn `UserConstructionScript`)
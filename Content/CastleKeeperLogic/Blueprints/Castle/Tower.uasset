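; Castle tower that fires a fireball at any actor entering its detection sphere, one shot per overlap.
; FireAtWill solves a ballistic toss from the sphere mesh or component to the target's current position at fixed launch speed, without tracing for obstacles.
; It spawns the projectile at half scale, applies that velocity and activates its movement component.
; Debug arc drawing and velocity printing are left on.
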(event `self.SphereCollision.OnComponentBeginOverlap`
  (params (OverlappedComponent :type "PrimitiveComponent Object Reference") (OtherActor :type "Actor Object Reference") (OtherComp :type "PrimitiveComponent Object Reference") (OtherBodyIndex :type Integer) (bFromSweep :type Boolean) (SweepResult :type "HitResult Structure (by ref)"))
  (`self.FireAtWill` OtherActor (`self.Fireball_BP`)))

(fn `FireAtWill`
  (params (TargetActor :type "Actor Object Reference") (Projectile_BP :type "/Game/CastleKeeperLogic/Blueprints/Castle/FireBall Class Reference"))
  (bind _returnvalue (`SceneComponent.K2_GetComponentLocation` (`self.Sphere`)))
  (bind _tossvelocity (`GameplayStatics.BlueprintSuggestProjectileVelocity` _returnvalue (`self.K2_GetActorLocation` TargetActor) 800.0 0.0 "DoNotTrace" 1.0 false true))
  (`KismetSystemLibrary.PrintString` (`KismetStringLibrary.Conv_VectorToString` _tossvelocity))
  (bind _returnvalue_2 (`|SpawnActorFromClass` Projectile_BP (`KismetMathLibrary.Conv_VectorToTransform` _returnvalue) "Undefined" "OverrideRootScale" null null))
  (bind _returnvalue_3 (`self.GetComponentByClass` _returnvalue_2 "/Script/Engine.ProjectileMovementComponent"))
  (`ProjectileMovementComponent.SetVelocityInLocalSpace` _returnvalue_3 _tossvelocity)
  (`self.SetActorScale3D` _returnvalue_2 (0.5 0.5 0.5))
  (`ActorComponent.Activate` _returnvalue_3 false))

(fn `UserConstructionScript`)
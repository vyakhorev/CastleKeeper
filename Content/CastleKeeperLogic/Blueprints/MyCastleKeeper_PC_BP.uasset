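; Player controller for Castle Keeper that places towers on the grid with the mouse.
; A left click traces under the cursor on the Visibility channel and, if it hits a Grid_Bp, spawns a BasicTower_BP at the exact hit location.
; Disconnected leftover logic holds a timed Rand_Sprite_BP spawner at the cursor and a debug line trace from the pawn camera, neither of which runs.
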(event `Key|LeftMouseButton`
  (params (Key :type "Key Structure"))
  (bind (_bblockinghit _binitialoverlap _time _location _impactpoint _normal _impactnormal _physmat _hitactor) (`GameplayStatics.BreakHitResult` (`self.GetHitResultUnderCursorByChannel` (`GameplayStatics.GetPlayerController` 0) "TraceTypeQuery1" true)))
  (:`Pressed`
    (cast `/Game/CastleKeeperLogic/Blueprints/Grid_Bp` _hitactor)
    (`|SpawnActorFromClass` "/Game/CastleKeeperLogic/Blueprints/BasicTower_BP.BasicTower_BP_C" (`KismetMathLibrary.Conv_VectorToTransform` _location) "Undefined" "OverrideRootScale" null null)))

(event `self.ReceiveTick`
  (params (DeltaSeconds :type "Float (single-precision)")))

(fn `UserConstructionScript`)